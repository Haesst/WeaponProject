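; BP_TargetDummy is a debug target dummy that shows feedback when it is hit.
; On begin play it shows its object name on a WBP_DummyInfo widget component.
; The DummyHit event replaces that text with the hit location and damage, then restores the name after a three-second delay.
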(event `self.ReceiveBeginPlay`
  (bind _output_get (set `self.DummyName` (`KismetSystemLibrary.GetObjectName` self)))
  (`self.Set DummyInfo Text` (`KismetTextLibrary.Conv_StringToText` _output_get)))

(event `DummyDamageInterface.DummyHit`
  (params (InDamage :type "Float (single-precision)") (HitLocation :type String))
  (`self.Set DummyInfo Text` (`KismetTextLibrary.Conv_StringToText` (`KismetStringLibrary.Concat_StrStr` "You hit: " (`KismetTextLibrary.Conv_TextToString` (`KismetTextLibrary.Conv_StringToText` HitLocation)) ", making " (`KismetStringLibrary.Conv_DoubleToString` InDamage) " damage"))
    (:`Out`
      (`KismetSystemLibrary.Delay` 3.0)
      (`self.Set DummyInfo Text` (`KismetTextLibrary.Conv_StringToText` (`self.DummyName`))))))

(fn `UserConstructionScript`)