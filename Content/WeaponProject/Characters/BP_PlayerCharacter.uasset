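; BP_PlayerCharacter is the player character Blueprint that handles weapon input for alternative fire and reload.
; Alternative fire is forwarded to CurrentWeapon, while the reload press calls CharacterReload through a DoOnce that resets on release.
; Primary fire and a camera-forward sphere trace that prints the hit actor's name are present but disconnected, so neither runs.
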(event `InputAction|AlternativeFire`
  (params (Key :type "Key Structure"))
  (:`Pressed`
    (`WeaponBase.OnAlternativeFire` (`self.CurrentWeapon`))))

(event `InputAction|Fire`
  (params (Key :type "Key Structure")))

(event `InputAction|Reload`
  (params (Key :type "Key Structure"))
  (:`Pressed`
    (`/Engine/EditorBlueprintResources/StandardMacros.DoOnce` false :!label _label
      (:`Completed`
        (`self.CharacterReload`))))
  (:`Released`
    (goto _label :!via `Reset`)))

(fn `UserConstructionScript`)